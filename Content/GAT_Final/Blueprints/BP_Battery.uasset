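; BP_Battery is a pickup that gives its Power value to the first-person character when overlapped.
; On overlap it calls PickupBattery on the character, then hides its mesh and disables its sphere collision instead of being destroyed.
; A timer set to RespawnTimer then shows the mesh and re-enables collision, so the battery respawns in place.
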(event Custom|RespawnBattery
  (Development|SetHiddeninGame (Variables|Default|GetStaticMesh) false false)
  (Collision|SetCollisionEnabled (Variables|Default|GetSphere) "QueryAndPhysics"))

(event EventBeginPlay)

(event Collision|EventActorBeginOverlap
  (params (OtherActor :type Actor%20Object%20Reference))
  (bind _asbp_first_person_character (Utilities|Casting|CastToBP_FirstPersonCharacter OtherActor))
  (Default|PickupBattery _asbp_first_person_character (Variables|Default|GetPower))
  (Development|SetHiddeninGame (Variables|Default|GetStaticMesh) true false)
  (Collision|SetCollisionEnabled (Variables|Default|GetSphere) "NoCollision")
  (Utilities|Time|SetTimerbyEvent (delegate Custom|RespawnBattery) (Variables|Default|GetRespawnTimer)))

(event EventTick
  (params (DeltaSeconds :type Float%20%28single-precision%29)))

(fn ConstructionScript)